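; Player controller that handles team choice and spawning as a team mothership.
; On BeginPlay the remote side shows a team selection widget, and TeamSelected stores the chosen team on the player state.
; ShowSpawnWidget then opens spawn selection for that team unless the game state reports an existing mothership.
; SpawnAsMothership forwards the spawn request to the game mode.
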(event `self.ReceiveBeginPlay`
  (`/Engine/EditorBlueprintResources/ActorMacros.Switch Has Authority`
    (:`Remote`
      (bind _returnvalue (`|CreateWidget` "/Game/Blueprints/Widgets/TeamSelectionWidget.TeamSelectionWidget_C"))
      (`UserWidget.AddToViewport` _returnvalue 0))))

(event `ShowSpawnWidget`
  (params (myTeam :type "/Game/Blueprints/Teams Enum" :default "NewEnumerator0"))
  (bind _asmy_first_game_state (cast `/Game/Blueprints/MyFirstGameState` (`GameplayStatics.GetGameState`)))
  (bind _mothershipexists (`/Game/Blueprints/MyFirstGameState.MothershipExists` _asmy_first_game_state myTeam))
  (if _mothershipexists
    (`KismetSystemLibrary.PrintString` "Mothership already exists")
    (else
      (bind _returnvalue (`|CreateWidget` "/Game/Blueprints/Widgets/SpawnSelectionWidget.SpawnSelectionWidget_C" null myTeam))
      (`UserWidget.AddToViewport` _returnvalue 0))))

(event `TeamSelected`
  (params (Team :type "/Game/Blueprints/Teams Enum" :default "NewEnumerator0") (Controller :type "/Game/Blueprints/MyFirstPlayerController Object Reference"))
  (bind _asmy_first_player_state (cast `/Game/Blueprints/MyFirstPlayerState` (`Controller.PlayerState` Controller)))
  (bind _output_get (set `/Game/Blueprints/MyFirstPlayerState.team` Team _asmy_first_player_state))
  (`self.ShowSpawnWidget` _output_get))

(event `SpawnAsMothership`
  (params (PlayerController :type "/Game/Blueprints/MyFirstPlayerController Object Reference") (Team :type "/Game/Blueprints/Teams Enum" :default "NewEnumerator0"))
  (bind _asmy_first_game_mode (cast `/Game/Blueprints/MyFirstGameMode` (`GameplayStatics.GetGameMode`)))
  (`/Game/Blueprints/MyFirstGameMode.SpawnAsMothership` _asmy_first_game_mode PlayerController Team))

(fn `UserConstructionScript`)