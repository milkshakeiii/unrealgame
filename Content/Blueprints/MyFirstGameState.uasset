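; MyFirstGameState is a game state Blueprint that reports whether a given team still has a mothership.
; MothershipExists scans all MyFirstPaperCharacter actors and returns true at the first one that is a mothership on that team, otherwise false.
; Each non-matching actor triggers an on-screen print of the queried team name, which looks like leftover debug output.
; The event graph and construction script are empty.
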(fn `MothershipExists`
  (params (forTeam :type "/Game/Blueprints/Teams Enum" :default "NewEnumerator0"))
  (returns (mothershipExists :type Boolean))
  (bind _outactors (`GameplayStatics.GetAllActorsOfClass` "/Game/Blueprints/Ships/MyFirstPaperCharacter.MyFirstPaperCharacter_C"))
  (for _array_element _outactors
    (bind _ismothership (`/Game/Blueprints/Ships/MyFirstPaperCharacter.IsMothership` _array_element))
    (if (and _ismothership (`|EnumEquality` (`/Game/Blueprints/Ships/MyFirstPaperCharacter.team` _array_element) forTeam))
      (return true)
      (else
        (`KismetSystemLibrary.PrintString` (`|GetEnumeratorNameAsString` forTeam)))))
  (return false))

(fn `UserConstructionScript`)