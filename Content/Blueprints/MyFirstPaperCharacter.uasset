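; Player-controlled Paper2D character that turns toward the mouse cursor, accelerates, brakes and fires projectiles.
; Input toggles scales that Tick feeds into movement input along actor forward (accelerate) or against velocity (brake).
; Rotation finds the shortest wrapped yaw difference to the cursor hit and adds proportional yaw input, unsigned below a small threshold.
; Fire spawns MyFirstProjectile at Arrow1 using the sprite's yaw.
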(event `InputAction|Brake`
  (params (Key :type "Key Structure"))
  (:`Pressed`
    (set `self.decelerationScale` 1.0))
  (:`Released`
    (set `self.decelerationScale` 0.0)))

(event `InputAction|Fire`
  (params (Key :type "Key Structure"))
  (:`Pressed`
    (`self.Fire`)))

(event `InputAction|Accelerate`
  (params (Key :type "Key Structure"))
  (:`Pressed`
    (set `self.accelerationScale` 1.0))
  (:`Released`
    (set `self.accelerationScale` 0.0)))

(event `self.ReceiveTick`
  (params (DeltaSeconds :type "Float (single-precision)"))
  (`self.Rotation` (`.Location` (`GameplayStatics.BreakHitResult` (`PlayerController.GetHitResultUnderCursorByChannel` (`GameplayStatics.GetPlayerController` 0) "TraceTypeQuery1" true))))
  (`self.Deceleration` (`self.decelerationScale`))
  (`self.Acceleration` (`self.accelerationScale`)))

(event `Fire`
  (`|SpawnActorFromClass` "/Game/Blueprints/MyFirstProjectile.MyFirstProjectile_C" (`KismetMathLibrary.MakeTransform` (`SceneComponent.K2_GetComponentLocation` (`self.Arrow1`)) (`KismetMathLibrary.MakeRotator` 90.0 0.0 (.yaw (`SceneComponent.K2_GetComponentRotation` (`self.PaperSprite`))))) "Undefined" "OverrideRootScale" null self))

(fn `Acceleration`
  (params (ScaleValue :type "Float (single-precision)"))
  ;[1 1 1] Acceleration
  (`self.AddMovementInput` (`self.GetActorForwardVector`) ScaleValue))

(fn `Deceleration`
  (params (ScaleValue :type "Float (single-precision)"))
  ;[1 1 1] Decleration
  (`self.AddMovementInput` (`KismetMathLibrary.RotateAngleAxis` (`self.GetVelocity`) 180.0 (0.0 0.0 1.0)) ScaleValue))

(fn `Rotation`
  (params (MouseWorldPosition :type "Vector Structure (by ref)"))
  (bind _yaw (.yaw (`self.K2_GetActorRotation`)))
  (bind _yaw_2 (.yaw (`KismetMathLibrary.FindLookAtRotation` (`self.K2_GetActorLocation`) MouseWorldPosition)))
  (bind _returnvalue (+ _yaw 0.0))
  (bind _returnvalue_2 (- _yaw 360.0))
  (bind _returnvalue_3 (+ _yaw 360.0))
  (bind _returnvalue_4 (`KismetMathLibrary.SelectFloat` (+ _yaw_2 360.0) _yaw_2 (< _yaw_2 0.0)))
  (bind _returnvalue_5 (`KismetMathLibrary.SelectFloat` _returnvalue_2 _returnvalue (< (`KismetMathLibrary.Abs` (- _returnvalue_2 _returnvalue_4)) (`KismetMathLibrary.Abs` (- _returnvalue _returnvalue_4)))))
  (bind _returnvalue_6 (`KismetMathLibrary.SelectFloat` _returnvalue_5 _returnvalue_3 (< (`KismetMathLibrary.Abs` (- _returnvalue_5 _returnvalue_4)) (`KismetMathLibrary.Abs` (- _returnvalue_3 _returnvalue_4)))))
  (bind _returnvalue_7 (`KismetMathLibrary.Abs` (- _returnvalue_6 _returnvalue_4)))
  (bind _returnvalue_8 (/ _returnvalue_7 100.0))
  ;[1 1 1] Rotate to face mouse cursor
  (`self.AddControllerYawInput` (`KismetMathLibrary.SelectFloat` _returnvalue_8 (* (`KismetMathLibrary.SelectFloat` 1.0 -1.0 (< _returnvalue_6 _returnvalue_4)) _returnvalue_8) (< _returnvalue_7 10.0))))

(fn `UserConstructionScript`)