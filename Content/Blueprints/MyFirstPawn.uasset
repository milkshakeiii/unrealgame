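; Player pawn that turns to face the mouse cursor, with input axes to accelerate and decelerate.
; Accelerate adds movement along the actor's forward vector, while Decelerate pushes opposite its velocity.
; Each Tick traces under the cursor and adds yaw input proportional to the shortest wrap-around angle to that point.
; Within a small angle threshold that input loses its sign and is never negative.
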(event `InputAxis|Decelerate`
  (params (AxisValue :type "Float (single-precision)"))
  ;[1 1 1] Decleration
  (`self.AddMovementInput` (`KismetMathLibrary.RotateAngleAxis` (`self.GetVelocity`) 180.0 (0.0 0.0 1.0)) AxisValue))

(event `InputAxis|Accelerate`
  (params (AxisValue :type "Float (single-precision)"))
  ;[1 1 1] Acceleration
  (`self.AddMovementInput` (`self.GetActorForwardVector`) AxisValue))

(event `self.ReceiveTick`
  (params (DeltaSeconds :type "Float (single-precision)"))
  (bind _yaw (.yaw (`self.K2_GetActorRotation`)))
  (bind _returnvalue (+ _yaw 0.0))
  (bind _returnvalue_2 (- _yaw 360.0))
  (bind _returnvalue_3 (+ _yaw 360.0))
  (bind _yaw_2 (.yaw (`KismetMathLibrary.FindLookAtRotation` (`self.K2_GetActorLocation`) (`.Location` (`GameplayStatics.BreakHitResult` (`PlayerController.GetHitResultUnderCursorByChannel` (`GameplayStatics.GetPlayerController` 0) "TraceTypeQuery1" true))))))
  (bind _returnvalue_4 (`KismetMathLibrary.SelectFloat` (+ _yaw_2 360.0) _yaw_2 (< _yaw_2 0.0)))
  (bind _returnvalue_5 (`KismetMathLibrary.SelectFloat` _returnvalue_2 _returnvalue (< (`KismetMathLibrary.Abs` (- _returnvalue_2 _returnvalue_4)) (`KismetMathLibrary.Abs` (- _returnvalue _returnvalue_4)))))
  (bind _returnvalue_6 (`KismetMathLibrary.SelectFloat` _returnvalue_5 _returnvalue_3 (< (`KismetMathLibrary.Abs` (- _returnvalue_5 _returnvalue_4)) (`KismetMathLibrary.Abs` (- _returnvalue_3 _returnvalue_4)))))
  (bind _returnvalue_7 (`KismetMathLibrary.Abs` (- _returnvalue_6 _returnvalue_4)))
  (bind _returnvalue_8 (/ _returnvalue_7 100.0))
  ;[1 1 1] Rotate to face mouse cursor
  (`self.AddControllerYawInput` (`KismetMathLibrary.SelectFloat` _returnvalue_8 (* (`KismetMathLibrary.SelectFloat` 1.0 -1.0 (< _returnvalue_6 _returnvalue_4)) _returnvalue_8) (< _returnvalue_7 10.0))))

(fn `UserConstructionScript`)